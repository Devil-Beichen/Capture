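; BP_围栏效果设置 is a fence effect setter that applies deletion or hit reactions to fence actors inside its Box volume.
; 循环检测 runs a near-zero-length multi box trace for WorldDynamic objects and returns the unique hit actors.
; 删除 sends those actors the 删除围栏 interface message, while 受击 sends 受击 with shake (晃动) and forward/reverse (正反) settings.
; The event graph and construction script are empty.
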(fn `UserConstructionScript`)

(fn `删除`
  (bind _hitactor (`self.循环检测`))
  (message `/Game/围栏/BP/BPI_围栏.删除围栏` _hitactor))

(fn `受击`
  (bind _hitactor (`self.循环检测`))
  (message `/Game/围栏/BP/BPI_围栏.受击` _hitactor (`self.晃动`) (`self.正反`)))

(fn `循环检测`
  (returns (HitActor :type "Array of Actor Object Reference"))
  (locals (TempLocalVar :type "Array of Actor Object Reference"))
  (bind _box (`self.Box`))
  (bind _templocalvar (`local.TempLocalVar`))
  (bind _returnvalue (`SceneComponent.K2_GetComponentLocation` _box))
  (bind (_outhits _returnvalue_2) (`KismetSystemLibrary.BoxTraceMultiForObjects` _returnvalue (+ _returnvalue (0.0 0.0 0.01)) (`BoxComponent.GetScaledBoxExtent` (`self.Box`)) (`SceneComponent.K2_GetComponentRotation` _box) (`|MakeArray` "ObjectTypeQuery2" :!type "EObjectTypeQuery Enum")))
  (if _returnvalue_2
    (for _array_element _outhits
      (`KismetArrayLibrary.Array_AddUnique` _templocalvar (`.HitActor` (`GameplayStatics.BreakHitResult` _array_element))))
    (return _templocalvar)
    (else
      (return))))