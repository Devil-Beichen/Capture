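; Wooden fence actor with a configurable mesh and a faction color, applied to its materials as the ZYColor vector parameter.
; The construction script sets the mesh and color, and BeginPlay caches the mesh's starting world scale.
; 显示 (show) unhides the fence if hidden and plays a sped-up timeline that scales the mesh relative to that cached scale.
; 变阵营 (change faction) recolors it and replays the same scale animation without changing visibility.
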(event `self.ReceiveBeginPlay`
  (set `self.StartScale` (`SceneComponent.K2_GetComponentScale` (`self.StaticMesh`))))

(event `显示`
  (if (`self.bHidden`)
    (`self.SetActorHiddenInGame` false)
    (`TimelineComponent.SetPlayRate` (`self.SetScale`) (/ 1.0 0.3) :!label _label)
    (bind (_direction _time) (`Timeline|SetScale` :!via `PlayFromStart`)
      (:`Update`
        (`SceneComponent.SetWorldScale3D` (`self.StaticMesh`) (* _time (`self.StartScale`)))))))

(event `变阵营`
  (params (Color1 :type "LinearColor Structure"))
  (bind _output_get (set `self.Color` Color1))
  (`MeshComponent.SetVectorParameterValueOnMaterials` (`self.StaticMesh`) "ZYColor" (`KismetMathLibrary.Conv_LinearColorToVector` _output_get))
  (goto _label))

(fn `UserConstructionScript`
  (`StaticMeshComponent.SetStaticMesh` (`self.StaticMesh`) (`self.模型`))
  (`MeshComponent.SetVectorParameterValueOnMaterials` (`self.StaticMesh`) "ZYColor" (`KismetMathLibrary.Conv_LinearColorToVector` (`self.Color`))))