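; Spline-based fence (围栏) that repeats a list of meshes along a spline, spaced by mesh bounds, scale and gap, with a shared color.
; The construction script lays them out as HISM instances for preview.
; On BeginPlay, 生成 spawns attached BP_木栏 actors at those points, optionally hidden, then clears the instances.
; Events destroy all pieces or run a looping timer, apparently to reveal them sequentially along the spline.
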(event `self.ReceiveBeginPlay`
  (`self.生成`))

(event `删除所有的`
  (for _array_element (`self.围栏`)
    (`/Engine/EditorBlueprintResources/StandardMacros.IsValid` _array_element
      (:`Is Valid`
        (`self.K2_DestroyActor` _array_element)))))

(event `开始持续显示`
  (`KismetArrayLibrary.Array_Clear` (`self.显示用的围栏`))
  (bind _output_get (set `self.显示用的围栏` (`self.围栏`)))
  (`KismetArrayLibrary.Array_Reverse` _output_get)
  (bind _returnvalue (`KismetSystemLibrary.K2_SetTimerDelegate` (`|CreateDelegate` :!event `显示`) 0.1 true))
  (set `self.显示定时器` _returnvalue))

(event `停止显示`
  (bind `_显示定时器` (`self.显示定时器`))
  (`KismetSystemLibrary.K2_PauseTimerHandle` `_显示定时器`)
  (`KismetSystemLibrary.K2_ClearAndInvalidateTimerHandle` `_显示定时器`))

(event `显示`
  (bind `_显示编号` (`self.显示编号`))
  (bind `_显示用的围栏` (`self.显示用的围栏`))
  (bind _output (`|GetArrayItem` `_显示用的围栏` `_显示编号`))
  (if (> `_显示编号` (`KismetArrayLibrary.Array_Length` `_显示用的围栏`))
    (`self.停止显示`)
    (else
      (`/Engine/EditorBlueprintResources/StandardMacros.IsValid` _output
        (:`Is Valid`
          (`/Game/围栏/BP/BP_木栏.显示` _output)
          (`/Engine/EditorBlueprintResources/StandardMacros.IncrementInt` `_显示编号`))))))

(fn `Add`
  (locals (Num :type Integer) (TempTransform :type "Transform Structure") (`编号` :type Integer :default 0))
  (bind _staticmeshcomponents (`self.StaticMeshComponents`))
  (bind `_编号` (`local.编号`))
  (bind (_returnvalue_origin _returnvalue_boxextent) (`KismetMathLibrary.BreakBoxSphereBounds` (`StaticMesh.GetBounds` (`|GetArrayItem` (`self.模型`) (select `bool` (== `_编号` 0) :`false` (- `_编号` 1) :`true` (- (`local.Num`) 1))))))
  (`KismetArrayLibrary.Array_Clear` (`self.StaticMeshComponents`))
  (for _array_element _staticmeshcomponents
    (`InstancedStaticMeshComponent.ClearInstances` _array_element))
  (`KismetArrayLibrary.Array_Clear` _staticmeshcomponents)
  (if (`KismetArrayLibrary.Array_IsNotEmpty` (`self.模型`))
    (for _array_element_2 (`self.模型`)
      (bind _returnvalue (`AddComponent|NODE_AddHierarchicalInstancedStaticMeshComponent-0`))
      (`StaticMeshComponent.SetStaticMesh` _returnvalue _array_element_2)
      (`KismetArrayLibrary.Array_AddUnique` (`self.StaticMeshComponents`) _returnvalue)
      (`MeshComponent.SetVectorParameterValueOnMaterials` _returnvalue "ZYColor" (`KismetMathLibrary.Conv_LinearColorToVector` (`self.Color`))))
    (set `local.Num` (`KismetArrayLibrary.Array_Length` (`self.模型`)))
    (set `self.当前所在的距离` 0.0)
    (for _index (range (`self.生成数量`))
      (bind _returnvalue_2 (mod _index (`local.Num`)))
      (set `local.编号` _returnvalue_2)
      (bind _returnvalue_3 (== _index 0))
      (bind _output_get (set `self.当前所在的距离` (+ (+ (`self.当前所在的距离`) (select `bool` _returnvalue_3 :`false` (* (.x (* _returnvalue_boxextent 2.0)) (`self.Size`)))) (select `bool` _returnvalue_3 :`false` (`self.间隔`)))))
      (bind _output_get_2 (set `local.TempTransform` (`KismetMathLibrary.MakeTransform` (.location (`SplineComponent.GetTransformAtDistanceAlongSpline` (`self.Spline`) _output_get "Local" true)) (.rotation (`SplineComponent.GetTransformAtDistanceAlongSpline` (`self.Spline`) _output_get "Local" true)) (* (.scale (`SplineComponent.GetTransformAtDistanceAlongSpline` (`self.Spline`) _output_get "Local" true)) (`self.Size`)))))
      (`InstancedStaticMeshComponent.AddInstance` (`|GetArrayItem` (`self.StaticMeshComponents`) _returnvalue_2) _output_get_2 false))))

(fn `UserConstructionScript`
  (`self.Add`))

(fn `生成`
  (locals (`当前所在的距离` :type "Float (double-precision)") (Num :type Integer) (`编号` :type Integer) (TempTransform :type "Transform Structure"))
  (bind `_编号` (`local.编号`))
  (bind (_returnvalue_origin _returnvalue_boxextent) (`KismetMathLibrary.BreakBoxSphereBounds` (`StaticMesh.GetBounds` (`|GetArrayItem` (`self.模型`) (select `bool` (== `_编号` 0) :`false` (- `_编号` 1) :`true` (- (`local.Num`) 1))))))
  (bind _returnvalue_x (`KismetMathLibrary.BreakVector` (* _returnvalue_boxextent 2.0)))
  (set `local.Num` (`KismetArrayLibrary.Array_Length` (`self.模型`)))
  (set `local.当前所在的距离` 0.0)
  (for _index (range (`self.生成数量`))
    (set `local.编号` (mod _index (`local.Num`)))
    (bind _returnvalue (== _index 0))
    (bind _output_get (set `local.当前所在的距离` (+ (+ (`local.当前所在的距离`) (select `bool` _returnvalue :`false` (* _returnvalue_x (`self.Size`)))) (select `bool` _returnvalue :`false` (`self.间隔`)))))
    (bind _output_get_2 (set `local.TempTransform` (`KismetMathLibrary.MakeTransform` (.location (`SplineComponent.GetTransformAtDistanceAlongSpline` (`self.Spline`) _output_get "World" true)) (.rotation (`SplineComponent.GetTransformAtDistanceAlongSpline` (`self.Spline`) _output_get "World" true)) (* (.scale (`SplineComponent.GetTransformAtDistanceAlongSpline` (`self.Spline`) _output_get "World" true)) (`self.Size`)))))
    (bind _returnvalue_2 (`|SpawnActorFromClass` "/Game/围栏/BP/BP_木栏.BP_木栏_C" _output_get_2 "AlwaysSpawn" "MultiplyWithRoot" self (`|GetArrayItem` (`self.模型`) (`local.编号`)) (`self.Color`) null))
    (`self.K2_AttachToComponent` _returnvalue_2 (`self.Spline`) "None" "KeepWorld" "KeepWorld" "KeepWorld" true)
    (`/Engine/EditorBlueprintResources/StandardMacros.IsValid` _returnvalue_2
      (:`Is Valid`
        (`KismetArrayLibrary.Array_AddUnique` (`self.围栏`) _returnvalue_2)
        (`self.SetActorHiddenInGame` _returnvalue_2 (`self.生成隐藏`)))))
  (`KismetArrayLibrary.Array_Reverse` (`self.围栏`))
  (for _array_element (`self.StaticMeshComponents`)
    (`InstancedStaticMeshComponent.ClearInstances` _array_element)))