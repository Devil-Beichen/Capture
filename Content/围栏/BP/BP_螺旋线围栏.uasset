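; Spiral fence roll that visually unrolls into a linked target fence (目标围栏) as 进度 increases.
; Construction grows a spiral spline to fit the piece count, taken from the target when valid, and previews meshes with HISMs.
; BeginPlay replaces the preview with attached BP_木栏 actors.
; Once 开始设置 is set, Tick shifts and rotates the spline to mimic rolling, hiding outer pieces while revealing their target-fence counterparts.
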(event `self.ReceiveBeginPlay`
  (`self.生成`))

(event `self.ReceiveTick`
  (params (DeltaSeconds :type "Float (single-precision)"))
  (bind `_上下` (`self.上下`))
  (bind (_returnvalue_x _returnvalue_y) (`KismetMathLibrary.BreakVector` (`SplineComponent.GetLocationAtTime` (`self.Spline`) (`KismetMathLibrary.Lerp` 1.0 0.0 (`self.进度`)) "Local" true)))
  (if (`self.开始设置`)
    (`SceneComponent.K2_SetRelativeLocationAndRotation` (`self.Spline`) (`KismetMathLibrary.MakeVector` (* (`KismetMathLibrary.Sqrt` (+ (`KismetMathLibrary.Square` _returnvalue_x) (`KismetMathLibrary.Square` _returnvalue_y))) (select `bool` `_上下` :`false` -1.0 :`true` 1.0))) (`KismetMathLibrary.MakeRotator` 0.0 0.0 (+ (* (`KismetMathLibrary.DegAtan2` _returnvalue_y _returnvalue_x) -1.0) (select `bool` `_上下` :`true` 180.0))) false false)
    (`self.隐藏`)))

(fn `Add`
  (locals (Num :type Integer :default 0) (`预想长度` :type "Float (double-precision)") (`当前所在的距离` :type "Float (double-precision)") (Indix :type Integer) (`角度` :type "Float (double-precision)"))
  (bind _boxextent_x (`KismetMathLibrary.BreakVector` (`self.Get Mesh Length` 0)))
  (bind _staticmeshcomponents (`self.StaticMeshComponents`))
  (bind `_预想长度` (`local.预想长度`))
  (bind `_角度` (`local.角度`))
  (bind `_上下` (`self.上下`))
  (bind _points (`self.Points`))
  (bind _returnvalue (+ (`self.螺旋线到中心的距离`) (* (`self.螺旋线的间距`) `_角度`)))
  (bind _x (.x (`|GetArrayItem` _points (`KismetArrayLibrary.Array_LastIndex` _points))))
  (bind _y (.y (`|GetArrayItem` _points (`KismetArrayLibrary.Array_LastIndex` _points))))
  (bind `_目标围栏` (`self.目标围栏`)
    (:`then`
      (set `self.生成数量` (`/Game/围栏/BP/BP_Spline_围栏.生成数量` `_目标围栏`)))
    (:`else`
      _))
  (for _array_element _staticmeshcomponents
    (`InstancedStaticMeshComponent.ClearInstances` _array_element))
  (`KismetArrayLibrary.Array_Clear` _staticmeshcomponents)
  (`KismetArrayLibrary.Array_Clear` (`self.Points`))
  (set `local.Num` (`KismetArrayLibrary.Array_Length` (`self.模型`)))
  (if (and (> (`self.生成数量`) 0) (`KismetArrayLibrary.Array_IsNotEmpty` (`self.模型`)))
    (for _array_element_2 (`self.模型`)
      (bind _returnvalue_2 (`AddComponent|NODE_AddHierarchicalInstancedStaticMeshComponent-0`))
      (`StaticMeshComponent.SetStaticMesh` _returnvalue_2 _array_element_2)
      (`KismetArrayLibrary.Array_AddUnique` (`self.StaticMeshComponents`) _returnvalue_2)
      (`SceneComponent.K2_AttachToComponent` _returnvalue_2 (`self.Spline`) "None" "KeepWorld" "KeepWorld" "KeepWorld" true)
      (`MeshComponent.SetVectorParameterValueOnMaterials` _returnvalue_2 "ZYColor" (`KismetMathLibrary.Conv_LinearColorToVector` (`self.Color`))))
    (set `local.预想长度` 0.0)
    (for _index (range (`self.生成数量`))
      (bind _returnvalue_3 (mod _index (`local.Num`)))
      (bind _boxextent_x_2 (`KismetMathLibrary.BreakVector` (`self.Get Mesh Length` (select `bool` (== _returnvalue_3 0) :`false` (- _returnvalue_3 1) :`true` (- (`local.Num`) 1)))))
      (set `local.预想长度` (+ (`local.预想长度`) (select `bool` (== _index 0) :`false` _boxextent_x_2 :`true` _boxextent_x))))
    (set `self.实际长度` `_预想长度`)
    (set `local.Indix` 0)
    (while (< (`SplineComponent.GetSplineLength` (`self.Spline`)) `_预想长度`)
      (set `local.角度` (* (* (`self.点间隔`) (select `bool` (`self.上下`) :`false` -1.0 :`true` 1.0)) (`local.Indix`)))
      (`KismetArrayLibrary.Array_Add` (`self.Points`) (`KismetMathLibrary.MakeVector` (* _returnvalue (`KismetMathLibrary.DegCos` `_角度`)) (* _returnvalue (`KismetMathLibrary.DegSin` `_角度`))))
      (`/Engine/EditorBlueprintResources/StandardMacros.IncrementInt` (`local.Indix`)
        (:`  `
          (`SplineComponent.SetSplinePoints` (`self.Spline`) (`self.Points`) "Local" true))))
    (`SceneComponent.K2_SetRelativeLocationAndRotation` (`self.Spline`) (`KismetMathLibrary.MakeVector` (* (`KismetMathLibrary.Sqrt` (+ (`KismetMathLibrary.Square` _x) (`KismetMathLibrary.Square` _y))) (select `bool` `_上下` :`false` -1.0 :`true` 1.0))) (`KismetMathLibrary.MakeRotator` 0.0 0.0 (+ (* (`KismetMathLibrary.DegAtan2` _y _x) -1.0) (select `bool` `_上下` :`true` 180.0))) false false)
    (bind _temptransforms (`self.Get Temp Transforms`))
    (for (_array_element_3 _array_index) _temptransforms
      (`InstancedStaticMeshComponent.AddInstance` (`|GetArrayItem` (`self.StaticMeshComponents`) (mod _array_index (`local.Num`))) _array_element_3 true))))

(fn `Get Mesh Length`
  (params (Index :type Integer))
  (returns (BoxExtent :type "Vector Structure"))
  (bind _output (`|GetArrayItem` (`self.模型`) Index))
  (bind (_returnvalue_origin _returnvalue_boxextent) (`KismetMathLibrary.BreakBoxSphereBounds` (`StaticMesh.GetBounds` _output)))
  (`/Engine/EditorBlueprintResources/StandardMacros.IsValid` _output
    (:`Is Valid`
      (return (* _returnvalue_boxextent 2.0 (`self.Size`))))
    (:`Is Not Valid`
      (return (0.0 0.0 0.0)))))

(fn `Get Temp Transforms`
  (returns (TempTransforms :type "Array of Transform Structure"))
  (locals (Num :type Integer) (`编号` :type Integer) (TempTransform :type "Array of Transform Structure") (`当前在的临时距离` :type "Float (double-precision)"))
  (bind `_编号` (`local.编号`))
  (bind _boxextent_x (`KismetMathLibrary.BreakVector` (`self.Get Mesh Length` (select `bool` (== `_编号` 0) :`false` (- `_编号` 1) :`true` (- (`local.Num`) 1)))))
  (set `local.Num` (`KismetArrayLibrary.Array_Length` (`self.模型`)))
  (`KismetArrayLibrary.Array_Clear` (`local.TempTransform`))
  (set `local.当前在的临时距离` 0.0)
  (for _index (range (`self.生成数量`))
    (set `local.编号` (mod _index (`local.Num`)))
    (bind _returnvalue (== _index 0))
    (bind _output_get (set `local.当前在的临时距离` (+ (+ (`local.当前在的临时距离`) (select `bool` _returnvalue :`false` _boxextent_x)) (select `bool` _returnvalue :`false` (`self.间隔`)))))
    (`KismetArrayLibrary.Array_AddUnique` (`local.TempTransform`) (`KismetMathLibrary.MakeTransform` (.location (`SplineComponent.GetTransformAtDistanceAlongSpline` (`self.Spline`) (- (`SplineComponent.GetSplineLength` (`self.Spline`)) _output_get) "World" true)) (`KismetMathLibrary.MakeRotator` (.roll (.rotation (`SplineComponent.GetTransformAtDistanceAlongSpline` (`self.Spline`) (- (`SplineComponent.GetSplineLength` (`self.Spline`)) _output_get) "World" true))) (.pitch (.rotation (`SplineComponent.GetTransformAtDistanceAlongSpline` (`self.Spline`) (- (`SplineComponent.GetSplineLength` (`self.Spline`)) _output_get) "World" true))) (+ (.yaw (.rotation (`SplineComponent.GetTransformAtDistanceAlongSpline` (`self.Spline`) (- (`SplineComponent.GetSplineLength` (`self.Spline`)) _output_get) "World" true))) 180.0)) (* (.scale (`SplineComponent.GetTransformAtDistanceAlongSpline` (`self.Spline`) (- (`SplineComponent.GetSplineLength` (`self.Spline`)) _output_get) "World" true)) (`self.Size`)))))
  (return (`local.TempTransform`)))

(fn `UserConstructionScript`
  (`self.Add`))

(fn `生成`
  (locals (`当前所在的距离` :type "Float (double-precision)") (Num :type Integer) (TempTransform :type "Transform Structure"))
  (set `local.Num` (`KismetArrayLibrary.Array_Length` (`self.模型`)))
  (bind _temptransforms (`self.Get Temp Transforms`))
  (for (_array_element _array_index) _temptransforms
    (bind _returnvalue (`|SpawnActorFromClass` "/Game/围栏/BP/BP_木栏.BP_木栏_C" _array_element "AlwaysSpawn" "MultiplyWithRoot" self (`|GetArrayItem` (`self.模型`) (mod _array_index (`local.Num`))) (`self.Color`) null))
    (`self.K2_AttachToComponent` _returnvalue (`self.Spline`) "None" "KeepWorld" "KeepWorld" "KeepWorld" true)
    (`/Engine/EditorBlueprintResources/StandardMacros.IsValid` _returnvalue
      (:`Is Valid`
        (`KismetArrayLibrary.Array_AddUnique` (`self.围栏`) _returnvalue))))
  (`KismetArrayLibrary.Array_Reverse` (`self.围栏`))
  (for _array_element_2 (`self.StaticMeshComponents`)
    (`InstancedStaticMeshComponent.ClearInstances` _array_element_2)))

(fn `隐藏`
  (locals (`当前所在的距离` :type "Float (double-precision)") (`编号` :type Integer) (Num :type Integer))
  (if (> (`self.进度`) 0.0)
    (set `local.当前所在的距离` 0.0)
    (for (_array_element _array_index) (`self.围栏`)
      (`|ExecutionSequence`
        (:`then_0`
          (bind (_returnvalue_origin _returnvalue_boxextent) (`KismetMathLibrary.BreakBoxSphereBounds` (`StaticMesh.GetBounds` (`/Game/围栏/BP/BP_木栏.模型` _array_element))))
          (bind _returnvalue_x (`KismetMathLibrary.BreakVector` (* _returnvalue_boxextent 2.0)))
          (bind _returnvalue (+ (`local.当前所在的距离`) (* _returnvalue_x (`self.Size`))))
          (bind _returnvalue_2 (>= _returnvalue (* (`SplineComponent.GetSplineLength` (`self.Spline`)) (- 1.0 (`self.进度`)))))
          (`self.SetActorHiddenInGame` _array_element _returnvalue_2))
        (:`then_1`
          (`self.SetActorHiddenInGame` (`|GetArrayItem` (`/Game/围栏/BP/BP_Spline_围栏.围栏` (`self.目标围栏`)) _array_index) (not _returnvalue_2)))
        (:`then_2`
          (set `local.当前所在的距离` _returnvalue))))
    (else
      (for _array_element_2 (`self.围栏`)
        (`self.SetActorHiddenInGame` _array_element_2 (`self.bHidden`))))))