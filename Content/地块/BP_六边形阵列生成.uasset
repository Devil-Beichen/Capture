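; Hex tile grid generator that spawns BP_六边形功能 actors and assigns them to regions.
; Construction Script computes staggered cell transforms into ST位置, adding child-actor previews and optional index labels.
; BeginPlay replaces previews with tiles, passing each a height offset sphere-traced from "地形"-tagged terrain, then applies starting regions after a short delay.
; 新增区域 reassigns regions later, finding tiles by row/column through 寻找对象, optionally skipping the transition animation.
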(event `self.ReceiveBeginPlay`
  (bind _returnvalue (`self.GetTransform`))
  (bind `_参照组件` (`self.参照组件`))
  (bind `_text组件` (`self.Text组件`))
  (bind `_六边形功能` (`self.六边形功能`))
  (for _array_element `_参照组件`
    (`/Engine/EditorBlueprintResources/StandardMacros.IsValid` _array_element
      (:`Is Valid`
        (`ActorComponent.K2_DestroyComponent` _array_element))))
  (`KismetArrayLibrary.Array_Clear` `_参照组件`)
  (for _array_element_2 `_text组件`
    (`/Engine/EditorBlueprintResources/StandardMacros.IsValid` _array_element_2
      (:`Is Valid`
        (`ActorComponent.K2_DestroyComponent` _array_element_2))))
  (`KismetArrayLibrary.Array_Clear` `_text组件`)
  (for (_array_element_3 _array_index) (`self.ST_位置`)
    (for (_array_element_4 _array_index_2) (`.位置_3_536974624EB482A3C7320C90D74734C9` (break `/Game/地块/ST_位置` _array_element_3))
      (bind _returnvalue_2 (`KismetMathLibrary.TransformLocation` _returnvalue (.location _array_element_4)))
      (bind _returnvalue_3 (`|SpawnActorFromClass` "/Game/地块/BP_六边形功能.BP_六边形功能_C" (`KismetMathLibrary.MakeTransform` (- _returnvalue_2 (0.0 0.0 100.0)) (`KismetMathLibrary.TransformRotation` _returnvalue (.rotation _array_element_4)) (.scale _array_element_4)) "AlwaysSpawn" "OverrideRootScale" null _array_index _array_index_2 self (`self.区域和颜色`) 0.3 (`KismetMathLibrary.Abs` (- (.z (`self.贴合地形` _returnvalue_2)) (.z (`self.K2_GetActorLocation`)))) null))
      (`KismetArrayLibrary.Array_Add` (`self.六边形功能`) _returnvalue_3))
    (`KismetArrayLibrary.Array_Add` (`self.六边形数组`) (make `/Game/地块/ST_六边形` `_六边形功能`))
    (`KismetArrayLibrary.Array_Clear` `_六边形功能`))
  (`KismetSystemLibrary.Delay` 0.2)
  (for _array_element_5 (`self.ST_开局存在区域`)
    (bind (`_区域编号` `_区域数组`) (break `/Game/地块/ST_开局存在区域` _array_element_5))
    (for _array_element_6 `_区域数组`
      (bind (`_横` `_竖`) (break `/Game/地块/ST_Index` _array_element_6))
      (bind `_六边形` (`self.寻找对象` `_横` `_竖`))
      (`/Engine/EditorBlueprintResources/StandardMacros.IsValid` `_六边形`
        (:`Is Valid`
          (`/Game/地块/BP_六边形功能.改变区域` `_六边形` true `_区域编号`))))))

(event `新增区域`
  (params (`新区域` :type "Array of /Game/地块/ST_开局存在区域 Structure") (`关闭变化过程动画` :type Boolean))
  (for _array_element `新区域`
    (bind (`_区域编号` `_区域数组`) (break `/Game/地块/ST_开局存在区域` _array_element))
    (for _array_element_2 `_区域数组`
      (bind (`_横` `_竖`) (break `/Game/地块/ST_Index` _array_element_2))
      (bind `_六边形` (`self.寻找对象` `_横` `_竖`))
      (`/Engine/EditorBlueprintResources/StandardMacros.IsValid` `_六边形`
        (:`Is Valid`
          (`/Game/地块/BP_六边形功能.改变区域` `_六边形` `关闭变化过程动画` `_区域编号`))))))

(fn `UserConstructionScript`
  (bind _staticinstance (`self.StaticInstance`))
  (bind `_参照组件` (`self.参照组件`))
  (bind `_中间缝隙` (`self.中间缝隙`))
  (bind `_text组件` (`self.Text组件`))
  (bind (_x _y) (`KismetMathLibrary.BreakVector2D` (`self.横列`)))
  (bind _returnvalue (* (`self.六边形大小`) (`self.宽度`)))
  (bind _returnvalue_2 (* (`self.六边形大小`) (`self.高度`)))
  (bind _returnvalue_3 (/ _returnvalue_2 2.0))
  (`/Engine/EditorBlueprintResources/StandardMacros.IsValid` _staticinstance
    (:`Is Valid`
      (`InstancedStaticMeshComponent.ClearInstances` _staticinstance))
    (:`Is Not Valid`
      _))
  (for _array_element `_text组件`
    (`/Engine/EditorBlueprintResources/StandardMacros.IsValid` _array_element
      (:`Is Valid`
        (`ActorComponent.K2_DestroyComponent` _array_element))))
  (`KismetArrayLibrary.Array_Clear` `_text组件`)
  (for _array_element_2 `_参照组件`
    (`/Engine/EditorBlueprintResources/StandardMacros.IsValid` _array_element_2
      (:`Is Valid`
        (`ActorComponent.K2_DestroyComponent` _array_element_2))))
  (`KismetArrayLibrary.Array_Clear` `_参照组件`)
  (bind _returnvalue_4 (`AddComponent|NODE_AddInstancedStaticMeshComponent-0` :`RelativeTransform` (`KismetMathLibrary.MakeTransform` (0.0 0.0 0.0))))
  (set `self.StaticInstance` _returnvalue_4)
  (for _index (range (`KismetMathLibrary.FTrunc` _x))
    (set `self.向上？` false)
    (`KismetArrayLibrary.Array_Clear` (`self.位置`))
    (for _index_2 (range (`KismetMathLibrary.FTrunc` _y))
      (set `self.向上？` (not (`self.向上？`)))
      (bind _returnvalue_5 (`KismetMathLibrary.MakeTransform` (`KismetMathLibrary.MakeVector` (- (- (+ (`KismetMathLibrary.SelectFloat` _returnvalue_3 0.0 (`self.向上？`)) (- 0.0 (* _returnvalue_2 _index))) (* `_中间缝隙` _index)) _returnvalue_3) (+ (* _index_2 (+ (/ _returnvalue 4.0) (/ _returnvalue 2.0))) (* `_中间缝隙` _index_2))) (struct :`Yaw` -90.0) (`KismetMathLibrary.Conv_DoubleToVector` (`self.六边形大小`))))
      (`KismetArrayLibrary.Array_Add` (`self.位置`) _returnvalue_5)
      (bind _returnvalue_6 (`AddComponent|NODE_AddChildActorComponent-0` :`RelativeTransform` _returnvalue_5))
      (if (`self.是否显示文本`)
        (bind _returnvalue_7 (`AddComponent|NODE_AddTextRenderComponent-0` :`RelativeTransform` (`KismetMathLibrary.MakeTransform` (+ (.location _returnvalue_5) (0.0 0.0 10.0)) (struct :`Pitch` 90.0 :`Yaw` 180.0))))
        (`TextRenderComponent.K2_SetText` _returnvalue_7 (`|FormatText` "{A}  {B}" (`KismetStringLibrary.Conv_IntToString` _index) (`KismetStringLibrary.Conv_IntToString` _index_2))))
      (`KismetArrayLibrary.Array_Add` (`self.Text组件`) _returnvalue_7)
      (`KismetArrayLibrary.Array_Add` (`self.参照组件`) _returnvalue_6))
    (`KismetArrayLibrary.Array_Add` (`self.ST_位置`) (make `/Game/地块/ST_位置` (`self.位置`)))))

(fn `寻找对象`
  (params (`横` :type Integer) (`竖` :type Integer))
  (returns (`六边形` :type "/Game/地块/BP_六边形功能 Object Reference"))
  (if (or (< `横` 0) (< `竖` 0))
    (return null)
    (else
      (return (`|GetArrayItem` (`.MemberVar_0_2_98B845E14CD5C03C799F10BB08129D0C` (break `/Game/地块/ST_六边形` (`|GetArrayItem` (`self.六边形数组`) `横`))) `竖`)))))

(fn `贴合地形`
  (params (Location :type "Vector Structure"))
  (returns (Return :type "Vector Structure"))
  (bind (_outhits _returnvalue) (`KismetSystemLibrary.SphereTraceMultiForObjects` (+ Location (0.0 0.0 1000.0)) (- Location (0.0 0.0 1000.0)) 100.0 (`|MakeArray` "ObjectTypeQuery1" :!type "EObjectTypeQuery Enum")))
  (if _returnvalue
    (for _array_element _outhits
      (bind (_bblockinghit _binitialoverlap _time _distance _location _impactpoint _normal _impactnormal _physmat _hitactor) (`GameplayStatics.BreakHitResult` _array_element))
      (if (`self.ActorHasTag` _hitactor "地形")
        (return _impactpoint)))))