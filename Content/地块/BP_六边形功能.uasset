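; Hex map tile that holds a region ID and shows region-colored border decals along the boundaries between regions.
; 改变区域 switches region, instantly at game start or with a timed scale and glow pulse.
; 改变 recolors edge materials, finds six neighbors through the generator using parity-based offsets, then calls 设置边缘.
; 设置边缘 hides both tiles' shared edges within a region, otherwise shows them and draws a debug arrow.
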(event `self.ReceiveBeginPlay`
  (bind `_区域和颜色` (`self.区域和颜色`))
  (bind _decal18 (`self.Decal18`))
  (bind `_区域和颜色_2` (`self.区域和颜色`))
  (`|ExecutionSequence`
    (:`then_0`
      (set `self.当前区域` 1)
      (set `self.Array` (`|MakeArray` (`self.SM_Select_02`) (`self.SM_Select_03`) (`self.SM_Select_04`) (`self.SM_Select_05`) (`self.SM_Select_06`) (`self.SM_Select_07`)))
      (for _array_element (`self.K2_GetComponentsByClass` "/Script/Engine.DecalComponent")
        (if (not (== _array_element (`self.Decal18`)))
          (`SceneComponent.SetHiddenInGame` _array_element true false)
          (bind _returnvalue (`DecalComponent.CreateDynamicMaterialInstance` _array_element))
          (`DecalComponent.SetDecalMaterial` _array_element _returnvalue)
          (`KismetArrayLibrary.Array_Add` (`self.边缘材质`) _returnvalue)
          (bind _keys (`BlueprintMapLibrary.Map_Keys` `_区域和颜色_2`))
          (bind _values (`BlueprintMapLibrary.Map_Values` `_区域和颜色_2`))
          (`MaterialInstanceDynamic.SetVectorParameterValue` _returnvalue "Color" (`|GetArrayItem` _values (`KismetArrayLibrary.Array_Find` _keys (`self.当前区域`)))))))
    (:`then_1`
      (bind _returnvalue_2 (`DecalComponent.CreateDynamicMaterialInstance` _decal18))
      (`DecalComponent.SetDecalMaterial` _decal18 _returnvalue_2)
      (bind _keys_2 (`BlueprintMapLibrary.Map_Keys` `_区域和颜色`))
      (bind _values_2 (`BlueprintMapLibrary.Map_Values` `_区域和颜色`))
      (`MaterialInstanceDynamic.SetVectorParameterValue` _returnvalue_2 "Color" (`|GetArrayItem` _values_2 (`KismetArrayLibrary.Array_Find` _keys_2 (`self.当前区域`)))))))

(event `改变区域`
  (params (`开局` :type Boolean) (`区域编号` :type Integer))
  (bind `_变化时间` (`self.变化时间`))
  (bind _beginscale (`self.BeginScale`))
  (bind `_区域和颜色` (`self.区域和颜色`))
  (if (not (== `区域编号` (`self.当前区域`)))
    (set `self.当前区域` `区域编号`)
    (if (not (`self.正在变换`))
      (set `self.正在变换` true)
      (bind _keys (`BlueprintMapLibrary.Map_Keys` `_区域和颜色`))
      (bind _values (`BlueprintMapLibrary.Map_Values` `_区域和颜色`))
      (set `self.颜色` (`|GetArrayItem` _values (`KismetArrayLibrary.Array_Find` _keys (`self.当前区域`))))
      (if `开局`
        (`self.改变`)
        (set `self.正在变换` false)
        (else
          (`|ExecutionSequence`
            (:`then_0`
              (`TimelineComponent.SetPlayRate` (`self.缩放T`) (/ 1.0 `_变化时间`))
              (set `self.BeginScale` (`self.GetActorScale3D`))
              (bind (_direction `_新建轨道_0`) (`Timeline|缩放T` :!via `PlayFromStart`)
                (:`Update`
                  (`self.SetActorScale3D` (`KismetMathLibrary.VLerp` _beginscale (* _beginscale 1.2) `_新建轨道_0`))
                  (for _array_element (`self.边缘材质`)
                    (`MaterialInstanceDynamic.SetScalarParameterValue` _array_element "自发光强度" (`KismetMathLibrary.Lerp` 1.0 (`KismetSystemLibrary.MakeLiteralDouble` (`self.最高亮度`)) `_新建轨道_0`))))
                (:`Finished`
                  (set `self.正在变换` false))))
            (:`then_1`
              (`self.改变`))
            (:`then_2`
              (`KismetSystemLibrary.K2_SetTimerDelegate` (delegate `改变`) (/ `_变化时间` 2.0)))))))))

(event `合并`
  (params (`合并边缘` :type Integer)))

(event `改变`
  (`SceneComponent.SetHiddenInGame` (`self.Decal18`) true false)
  (for _array_element (`self.K2_GetComponentsByClass` "/Script/Engine.DecalComponent")
    (if (not (== _array_element (`self.Decal18`)))
      (`SceneComponent.SetHiddenInGame` _array_element false false)))
  (for _array_element_2 (`self.边缘材质`)
    (`MaterialInstanceDynamic.SetVectorParameterValue` _array_element_2 "Color" (`self.颜色`)))
  (if (== (mod (`self.竖`) 2) 0)
    (`|ExecutionSequence`
      (:`then_0`
        (`self.设置边缘` 0 (`/Game/地块/BP_六边形阵列生成.寻找对象` (`self.生成器`) (- (`self.横`) 1) (- (`self.竖`) 1))))
      (:`then_1`
        (`self.设置边缘` 1 (`/Game/地块/BP_六边形阵列生成.寻找对象` (`self.生成器`) (- (`self.横`) 1) (`self.竖`))))
      (:`then_2`
        (`self.设置边缘` 2 (`/Game/地块/BP_六边形阵列生成.寻找对象` (`self.生成器`) (- (`self.横`) 1) (+ (`self.竖`) 1))))
      (:`then_3`
        (`self.设置边缘` 3 (`/Game/地块/BP_六边形阵列生成.寻找对象` (`self.生成器`) (`self.横`) (+ (`self.竖`) 1))))
      (:`then_4`
        (`self.设置边缘` 4 (`/Game/地块/BP_六边形阵列生成.寻找对象` (`self.生成器`) (+ (`self.横`) 1) (`self.竖`))))
      (:`then_5`
        (`self.设置边缘` 5 (`/Game/地块/BP_六边形阵列生成.寻找对象` (`self.生成器`) (`self.横`) (- (`self.竖`) 1)))))
    (else
      (`|ExecutionSequence`
        (:`then_0`
          (`self.设置边缘` 0 (`/Game/地块/BP_六边形阵列生成.寻找对象` (`self.生成器`) (`self.横`) (- (`self.竖`) 1))))
        (:`then_1`
          (`self.设置边缘` 1 (`/Game/地块/BP_六边形阵列生成.寻找对象` (`self.生成器`) (- (`self.横`) 1) (`self.竖`))))
        (:`then_2`
          (`self.设置边缘` 2 (`/Game/地块/BP_六边形阵列生成.寻找对象` (`self.生成器`) (`self.横`) (+ (`self.竖`) 1))))
        (:`then_3`
          (`self.设置边缘` 3 (`/Game/地块/BP_六边形阵列生成.寻找对象` (`self.生成器`) (+ (`self.横`) 1) (+ (`self.竖`) 1))))
        (:`then_4`
          (`self.设置边缘` 4 (`/Game/地块/BP_六边形阵列生成.寻找对象` (`self.生成器`) (+ (`self.横`) 1) (`self.竖`))))
        (:`then_5`
          (`self.设置边缘` 5 (`/Game/地块/BP_六边形阵列生成.寻找对象` (`self.生成器`) (+ (`self.横`) 1) (- (`self.竖`) 1))))))))

(fn `UserConstructionScript`
  (`|ExecutionSequence`))

(fn `设置边缘`
  (params (`判断边缘` :type Integer) (`边缘对象` :type "/Game/地块/BP_六边形功能 Object Reference"))
  (bind _returnvalue (`self.K2_GetActorLocation` `边缘对象`))
  (bind `_边缘对照表` (`self.边缘对照表`))
  (bind `_判断边缘` (`local.判断边缘`))
  (bind _output (`|GetArrayItem` (`self.Array`) `_判断边缘`))
  (`/Engine/EditorBlueprintResources/StandardMacros.IsValid` `边缘对象`
    (:`Is Valid`
      (bind _keys (`BlueprintMapLibrary.Map_Keys` `_边缘对照表`))
      (bind _values (`BlueprintMapLibrary.Map_Values` `_边缘对照表`))
      (if (== (`/Game/地块/BP_六边形功能.当前区域` `边缘对象`) (`self.当前区域`))
        (`SceneComponent.SetHiddenInGame` _output true true)
        (bind _output_2 (`|GetArrayItem` (`/Game/地块/BP_六边形功能.Array` `边缘对象`) (- (`|GetArrayItem` _values (`KismetArrayLibrary.Array_Find` _keys (+ `_判断边缘` 1))) 1)))
        (`SceneComponent.SetHiddenInGame` _output_2 true true)
        (return)
        (else
          (`|ExecutionSequence`
            (:`then_0`
              (`/Engine/EditorBlueprintResources/StandardMacros.IsValid` _output
                (:`Is Valid`
                  (`SceneComponent.SetHiddenInGame` _output false true))))
            (:`then_1`
              (`/Engine/EditorBlueprintResources/StandardMacros.IsValid` _output_2
                (:`Is Valid`
                  (`SceneComponent.SetHiddenInGame` _output_2 false true))))
            (:`then_2`
              (`KismetSystemLibrary.DrawDebugArrow` (+ _returnvalue (0.0 0.0 500.0)) (- _returnvalue (0.0 0.0 500.0)) 0.0 (struct) 3.0)
              (return))))))
    (:`Is Not Valid`
      (return))))

(fn `设置颜色和透明度`
  (params (`数据` :type "Map of LinearColor Structure to Float (double-precision)") (`材质实例` :type "MaterialInstanceDynamic Object Reference") (`Dimension 1` :type Integer))
  (bind _keys (`BlueprintMapLibrary.Map_Keys` `数据`))
  (`MaterialInstanceDynamic.SetVectorParameterValue` `材质实例` "color" (`|GetArrayItem` _keys `Dimension 1`))
  (bind _values (`BlueprintMapLibrary.Map_Values` `数据`))
  (`MaterialInstanceDynamic.SetScalarParameterValue` `材质实例` "不透明度" (`|GetArrayItem` _values `Dimension 1`)))

(fn `起始材质`
  (params (Array :type "Array of StaticMeshComponent Object Reference"))
  (bind `_区域和颜色` (`self.区域和颜色`))
  (for _array_element Array
    (bind _returnvalue (`PrimitiveComponent.CreateDynamicMaterialInstance` _array_element 0 (`PrimitiveComponent.GetMaterial` _array_element 0) "None"))
    (`PrimitiveComponent.SetMaterial` _array_element 0 _returnvalue)
    (`KismetArrayLibrary.Array_Add` (`self.边缘材质`) _returnvalue)
    (bind _keys (`BlueprintMapLibrary.Map_Keys` `_区域和颜色`))
    (bind _values (`BlueprintMapLibrary.Map_Values` `_区域和颜色`))
    (`MaterialInstanceDynamic.SetVectorParameterValue` _returnvalue "颜色" (`|GetArrayItem` _values (`KismetArrayLibrary.Array_Find` _keys (`self.当前区域`))))))