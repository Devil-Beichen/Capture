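; Dissolve volume actor that feeds a sphere or box shape's position and size into the MPC_溶解参数集 material parameter collection for dissolve materials.
; The S形状 enum picks one of three sphere or three box slots, setting the parameter names and which preview mesh and collision component is visible.
; SetValue resizes the components, then writes actor location plus scaled radius or full box size, from the construction script and every Tick.
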(event `self.ReceiveTick`
  (params (DeltaSeconds :type "Float (single-precision)"))
  (`self.SetValue`))

(fn `SetName`
  (switch `/Game/地形遮罩/溶解材质/BP/S_形状` (`self.S_形状`)
    (:`NewEnumerator0`
      (set `self.球体` true)
      (set `self.谁的位置` "圆形1位置")
      (set `self.谁的半径` "圆形1半径"))
    (:`NewEnumerator1`
      (set `self.球体` true)
      (set `self.谁的位置` "圆形2位置")
      (set `self.谁的半径` "圆形2半径"))
    (:`NewEnumerator4`
      (set `self.球体` true)
      (set `self.谁的位置` "圆形3位置")
      (set `self.谁的半径` "圆形3半径"))
    (:`NewEnumerator2`
      (set `self.球体` false)
      (set `self.谁的位置` "矩形1位置")
      (set `self.谁的半径` "矩形1大小"))
    (:`NewEnumerator3`
      (set `self.球体` false)
      (set `self.谁的位置` "矩形2位置")
      (set `self.谁的半径` "矩形2大小"))
    (:`NewEnumerator5`
      (set `self.球体` false)
      (set `self.谁的位置` "矩形3位置")
      (set `self.谁的半径` "矩形3大小")))
  (return))

(fn `SetSize`
  (bind _returnvalue (`self.GetActorScale3D`))
  (bind `_盒体大小` (`self.盒体大小`))
  (`SceneComponent.SetWorldScale3D` (`self.SphereMesh`) (* (`KismetMathLibrary.Conv_DoubleToVector` (/ (`self.半径`) 50.0)) _returnvalue))
  (`BoxComponent.SetBoxExtent` (`self.Box`) (* (50.0 50.0 50.0) `_盒体大小`) true)
  (`SceneComponent.SetWorldScale3D` (`self.Cube`) (* `_盒体大小` _returnvalue))
  (`SphereComponent.SetSphereRadius` (`self.Sphere`) (`self.半径`) true))

(fn `SetValue`
  (`self.SetSize`)
  (`self.SetName`)
  (if (`self.球体`)
    (`KismetMaterialLibrary.SetVectorParameterValue` "/Game/地形遮罩/溶解材质/MF/MPC_溶解参数集.MPC_溶解参数集" (`self.谁的位置`) (make `LinearColor` 0.0 0.0 0.0 1.0))
    (`KismetMaterialLibrary.SetVectorParameterValue` "/Game/地形遮罩/溶解材质/MF/MPC_溶解参数集.MPC_溶解参数集" (`self.谁的半径`) (make `LinearColor` 0.0 0.0 0.0 1.0))
    (`KismetMaterialLibrary.SetVectorParameterValue` "/Game/地形遮罩/溶解材质/MF/MPC_溶解参数集.MPC_溶解参数集" (`self.谁的位置`) (`KismetMathLibrary.Conv_VectorToLinearColor` (`self.K2_GetActorLocation`)))
    (`KismetMaterialLibrary.SetScalarParameterValue` "/Game/地形遮罩/溶解材质/MF/MPC_溶解参数集.MPC_溶解参数集" (`self.谁的半径`) (`SphereComponent.GetScaledSphereRadius` (`self.Sphere`)))
    (else
      (`KismetMaterialLibrary.SetVectorParameterValue` "/Game/地形遮罩/溶解材质/MF/MPC_溶解参数集.MPC_溶解参数集" (`self.谁的位置`) (make `LinearColor` 0.0 0.0 0.0 1.0))
      (`KismetMaterialLibrary.SetScalarParameterValue` "/Game/地形遮罩/溶解材质/MF/MPC_溶解参数集.MPC_溶解参数集" (`self.谁的半径`))
      (`KismetMaterialLibrary.SetVectorParameterValue` "/Game/地形遮罩/溶解材质/MF/MPC_溶解参数集.MPC_溶解参数集" (`self.谁的位置`) (`KismetMathLibrary.Conv_VectorToLinearColor` (`self.K2_GetActorLocation`)))
      (`KismetMaterialLibrary.SetVectorParameterValue` "/Game/地形遮罩/溶解材质/MF/MPC_溶解参数集.MPC_溶解参数集" (`self.谁的半径`) (`KismetMathLibrary.Conv_VectorToLinearColor` (* (`BoxComponent.GetScaledBoxExtent` (`self.Box`)) 2.0))))))

(fn `UserConstructionScript`
  (`self.SetValue`)
  (if (`self.球体`)
    (`SceneComponent.SetVisibility` (`self.Sphere`) true false)
    (`SceneComponent.SetVisibility` (`self.SphereMesh`) true false)
    (`SceneComponent.SetVisibility` (`self.Cube`) false false)
    (`SceneComponent.SetVisibility` (`self.Box`) false false)
    (else
      (`SceneComponent.SetVisibility` (`self.Cube`) true false)
      (`SceneComponent.SetVisibility` (`self.Box`) true false)
      (`SceneComponent.SetVisibility` (`self.Sphere`) false false)
      (`SceneComponent.SetVisibility` (`self.SphereMesh`) false false))))