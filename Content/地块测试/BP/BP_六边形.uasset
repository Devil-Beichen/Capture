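; Hex tile actor that finds its neighbors in the BP六边形阵列 grid and marks them with debug lines.
; 查找周围 derives six neighbor coordinates from its 编号, using offset coordinates where the parity of X shifts Y in adjacent rows.
; Debug resolves each coordinate through 寻找六边形 and briefly draws a vertical yellow line at any tile found.
; 测试 is a separate loop-based test of neighbor lookup with different index math.
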(event `查找周围`
  (bind (`_编号_x` `_编号_y`) (break `/Game/地块测试/BP/S_编号` (`self.编号`)))
  (bind (`_编号_x_2` `_编号_y_2`) (break `/Game/地块测试/BP/S_编号` (`self.编号`)))
  (bind (`_编号_x_3` `_编号_y_3`) (break `/Game/地块测试/BP/S_编号` (`self.编号`)))
  (bind _returnvalue (- `_编号_x` 1))
  (bind _returnvalue_2 (+ `_编号_x_2` 1))
  (bind _returnvalue_3 (== (mod `_编号_x_2` 2) 0))
  (bind _returnvalue_4 (== (mod `_编号_x` 2) 0))
  (`self.BP_六边形阵列`
    (:`then`
      (`|ExecutionSequence`
        (:`then_0`
          (`|ExecutionSequence`
            (:`then_0`
              (`self.Debug` (make `/Game/地块测试/BP/S_编号` _returnvalue_2 (select `bool` _returnvalue_3 :`false` `_编号_y_2` :`true` (- `_编号_y_2` 1)))))
            (:`then_1`
              (`self.Debug` (make `/Game/地块测试/BP/S_编号` _returnvalue_2 (select `bool` _returnvalue_3 :`false` (+ `_编号_y_2` 1) :`true` `_编号_y_2`))))))
        (:`then_1`
          (`|ExecutionSequence`
            (:`then_0`
              (`self.Debug` (make `/Game/地块测试/BP/S_编号` `_编号_x_3` (- `_编号_y_3` 1))))
            (:`then_1`
              (`self.Debug` (make `/Game/地块测试/BP/S_编号` `_编号_x_3` (+ `_编号_y_3` 1))))))
        (:`then_2`
          (`|ExecutionSequence`
            (:`then_0`
              (`self.Debug` (make `/Game/地块测试/BP/S_编号` _returnvalue (select `bool` _returnvalue_4 :`false` `_编号_y` :`true` (- `_编号_y` 1)))))
            (:`then_1`
              (`self.Debug` (make `/Game/地块测试/BP/S_编号` _returnvalue (select `bool` _returnvalue_4 :`false` (+ `_编号_y` 1) :`true` `_编号_y`))))))))
    (:`else`)))

(event `测试`
  (bind (`_编号_x` `_编号_y`) (break `/Game/地块测试/BP/S_编号` (`self.编号`)))
  (for _index (range -1 2)
    (for _index_2 (range 2)
      (`self.Debug` (make `/Game/地块测试/BP/S_编号` (+ _index `_编号_x`) (+ _index_2 (select `bool` (== _index 0) :`false` (- `_编号_y` 1) :`true` (select `bool` (== _index_2 1) :`false` 1 :`true` 2))))))))

(fn `Debug`
  (params (`寻找编号` :type "/Game/地块测试/BP/S_编号 Structure"))
  (bind `_bp_六边形阵列` (`self.BP_六边形阵列`)
    (:`then`
      (bind `_六边形` (`/Game/地块测试/BP/BP_六边形阵列.寻找六边形` `_bp_六边形阵列` `寻找编号`))
      (`/Engine/EditorBlueprintResources/StandardMacros.IsValid` `_六边形`
        (:`Is Valid`
          (bind _returnvalue (`self.K2_GetActorLocation` `_六边形`))
          (`KismetSystemLibrary.DrawDebugLine` (+ _returnvalue (0.0 0.0 100.0)) (- _returnvalue (0.0 0.0 100.0)) (struct :`R` 1.0 :`G` 1.0 :`A` 1.0) 1.0 1.0))))
    (:`else`)))

(fn `UserConstructionScript`)