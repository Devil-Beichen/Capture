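; Actor Blueprint that lays out a configurable hexagonal tile grid and can spawn functional tile actors on it.
; The construction script rebuilds HISM instances by row and column, offsetting odd rows half a width, with spacing from size, width and gap.
; It records each cell's coordinate ID and optionally adds row:column text labels.
; The 生成 event spawns a BP_六边形功能 at each instance's world transform, passing that ID.
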(event `生成`
  (for (_array_element _array_index) (`self.编号数组`)
    (`|SpawnActorFromClass` "/Game/地块测试/BP/BP_六边形功能.BP_六边形功能_C" (`InstancedStaticMeshComponent.GetInstanceTransform` (`self.HierarchicalInstancedStaticMesh`) _array_index true) "AlwaysSpawn" "MultiplyWithRoot" null _array_element null)))

(fn `AddHexagonalGround`
  (locals (TempTransform :type "Transform Structure"))
  (bind _newvar (`self.NewVar`))
  (bind _temptransform (`local.TempTransform`))
  (`InstancedStaticMeshComponent.ClearInstances` (`self.HierarchicalInstancedStaticMesh`))
  (for _array_element _newvar
    (`/Engine/EditorBlueprintResources/StandardMacros.IsValid` _array_element
      (:`Is Valid`
        (`ActorComponent.K2_DestroyComponent` _array_element))))
  (`KismetArrayLibrary.Array_Clear` _newvar)
  (`KismetArrayLibrary.Array_Clear` (`self.编号数组`))
  (for _index (range (`self.行`))
    (for _index_2 (range (`self.列`))
      (`KismetArrayLibrary.Array_AddUnique` (`self.编号数组`) (make `/Game/地块测试/BP/S_编号` _index _index_2))
      (set `local.TempTransform` (`KismetMathLibrary.MakeTransform` (`KismetMathLibrary.MakeVector` (* _index (* (`KismetMathLibrary.Sqrt` 3.0) (/ (`self.实际宽度`) 2.0))) (+ (* _index_2 (`self.实际宽度`)) (* (mod _index 2) (/ (`self.实际宽度`) 2.0)))) (struct) (`KismetMathLibrary.Conv_DoubleToVector` (`self.Szie`))))
      (`InstancedStaticMeshComponent.AddInstance` (`self.HierarchicalInstancedStaticMesh`) _temptransform false)
      (if (`self.显示行列`)
        (bind _returnvalue (`AddComponent|NODE_AddTextRenderComponent-0` :`RelativeTransform` (`KismetMathLibrary.MakeTransform` (.location _temptransform) (struct :`Pitch` 90.0 :`Yaw` 180.0) (/ (.scale _temptransform) 2.0))))
        (`TextRenderComponent.K2_SetText` _returnvalue (`|FormatText` "{行}:{列}" _index _index_2))
        (`KismetArrayLibrary.Array_AddUnique` (`self.NewVar`) _returnvalue)))))

(fn `UserConstructionScript`
  (`self.AddHexagonalGround`))

(fn `实际宽度`
  (returns (Value :type "Float (double-precision)"))
  (return (* (`self.Szie`) (+ (`self.宽度`) (`self.间隔`)))))